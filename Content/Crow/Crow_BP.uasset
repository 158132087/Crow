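; Player-controlled crow Character that switches between walking and flying.
; Movement input follows full control rotation in flight and only yaw otherwise.
; Falling or the Fly input starts flight with controller pitch; a short sphere trace from Arrow1 lands it through a DoOnce, re-armed after a delay following takeoff.
; FlyFast raises flight speed and widens camera FOV through a timeline, reversing it on release.
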(event Custom|Fly
  (bind _returnvalue (Transformation|GetActorRotation))
  (Pawn|Components|CharacterMovement|SetMovementMode (Variables|Character|GetCharacterMovement) "MOVE_Flying" 0)
  (Variables|Default|SetbUseControllerRotationPitch true)
  (Utilities|FlowControl|Delay 2.0)
  (Utilities|FlowControl|DoOnce false) ; enters at Reset
)

(event EventTick
  (params (DeltaSeconds :type Float%20%28single-precision%29))
  (bind _returnvalue (Transformation|GetActorRotation))
  (bind _arrow1 (Variables|Default|GetArrow1))
  (bind _returnvalue_2 (Transformation|GetWorldLocation _arrow1))
  (Utilities|FlowControl|Sequence
    (:then_0
      (bind _outhit (Collision|SphereTraceByChannel _returnvalue_2 (+ _returnvalue_2 (* (Math|Vector|GetForwardVector (Transformation|GetWorldRotation _arrow1)) 7.0)) 2e+01 "TraceTypeQuery3" false 0 "None"))
      (if (.bBlockingHit (Collision|BreakHitResult _outhit))
        (Utilities|FlowControl|DoOnce false
          (:Completed
            (Pawn|Components|CharacterMovement|SetMovementMode (Variables|Character|GetCharacterMovement) "MOVE_Walking" 0)
            (Variables|Default|SetbUseControllerRotationPitch false)
            (Transformation|SetActorRotation (Math|Rotator|MakeRotator (.roll _returnvalue) 0.0 (.yaw _returnvalue)))))))
    (:then_1
      (if (AI|Components|NavMovement|IsFalling (Variables|Character|GetCharacterMovement))
        (CallFunction|Fly)))))

(event Input|ActionEvents|InputActionFlyFast
  (params (Key :type Key%20Structure :default "None"))
  (bind _charactermovement (Variables|Character|GetCharacterMovement))
  (:Pressed
    (if (Utilities|Enum|Equal(Enum) (Variables|/Script/Engine.CharacterMovementComponent|GetMovementMode (Variables|Character|GetCharacterMovement)) "MOVE_Flying")
      (Variables|/Script/Engine.CharacterMovementComponent|SetMaxFlySpeed _charactermovement 8e+02)
      (bind _alpha (Timeline|时间轴_0 PlayFromStart)
        (:Update
          (Camera|SetFieldOfView (Variables|MyCharacter|GetFollowCamera) (Math|Float|Lerp 9e+01 135.0 _alpha))))))
  (:Released
    (Variables|/Script/Engine.CharacterMovementComponent|SetMaxFlySpeed _charactermovement 4e+02)
    (Timeline|时间轴_0 Reverse)))

(event Input|ActionEvents|InputActionFly
  (params (Key :type Key%20Structure :default "None"))
  (:Pressed
    (CallFunction|Fly)))

(event Input|AxisEvents|InputAxisLookUp
  (params (AxisValue :type Float%20%28single-precision%29))
  (Pawn|Input|AddControllerPitchInput AxisValue))

(event Input|AxisEvents|InputAxisTurn
  (params (AxisValue :type Float%20%28single-precision%29))
  (Pawn|Input|AddControllerYawInput AxisValue))

(event Input|AxisEvents|InputAxisMoveForward
  (params (AxisValue :type Float%20%28single-precision%29))
  (if (Utilities|Enum|Equal(Enum) (Variables|/Script/Engine.CharacterMovementComponent|GetMovementMode (Variables|Character|GetCharacterMovement)) "MOVE_Flying")
    (Pawn|Input|AddMovementInput (Math|Vector|GetForwardVector (Pawn|GetControlRotation :!class /Script/Engine.Pawn)) AxisValue false)
    (else
      (Pawn|Input|AddMovementInput (Math|Vector|GetForwardVector (Math|Rotator|MakeRotator 0.0 0.0 (.Yaw (Math|Rotator|BreakRotator (Pawn|GetControlRotation :!class /Script/Engine.Pawn))))) AxisValue false))))

(event Input|AxisEvents|InputAxisMoveRight
  (params (AxisValue :type Float%20%28single-precision%29))
  (if (Utilities|Enum|Equal(Enum) (Variables|/Script/Engine.CharacterMovementComponent|GetMovementMode (Variables|Character|GetCharacterMovement)) "MOVE_Flying")
    (Pawn|Input|AddMovementInput (Math|Vector|GetRightVector (Pawn|GetControlRotation :!class /Script/Engine.Pawn)) AxisValue false)
    (else
      (Pawn|Input|AddMovementInput (Math|Vector|GetRightVector (Math|Rotator|MakeRotator 0.0 0.0 (.Yaw (Math|Rotator|BreakRotator (Pawn|GetControlRotation :!class /Script/Engine.Pawn))))) AxisValue false))))

(fn ConstructionScript)